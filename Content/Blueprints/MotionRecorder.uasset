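; MotionRecorder captures head and hand motion as sequences of relative transforms and saves them through a MotionSaveSystem save game object.
; StartRecord opens a new sequence and a fixed-length timer that calls EndRecord to stop capture.
; While recording, Tick appends the current Head, LeftHand and RightHand transforms to the latest sequence, printing each sample to screen.
; SaveRecords passes all sequences and a file name to the save object created in the construction script.
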(event Custom|SaveRecords
  (Default|SaveMotion (Variables|Default|GetSaveMotion) (Variables|Default|Getsequences) (Variables|Default|GetsaveFileName)))

(event Custom|StartRecord
  (Variables|Default|SetIsRecordStarted true)
  (Utilities|Time|SetTimerbyEvent (delegate Custom|EndRecord) 1e+01)
  (Utilities|Array|Add (Variables|Default|Getsequences) (Utilities|Struct|MakeSequenceToSave)))

(event Custom|EndRecord
  (Variables|Default|SetIsRecordStarted false))

(event EventBeginPlay)

(event Collision|EventActorBeginOverlap
  (params (OtherActor :type Actor%20Object%20Reference)))

(event EventTick
  (params (DeltaSeconds :type Float%20%28single-precision%29))
  (bind _sequences (Variables|Default|Getsequences))
  (if (Variables|Default|GetIsRecordStarted)
    (bind _transforms (CallFunction|FetchCurrentTransforms))
    (Utilities|Array|Add (Utilities|Struct|BreakSequenceToSave (Utilities|Array|Get(acopy) _sequences (Utilities|Array|LastIndex _sequences))) _transforms)))

(fn ConstructionScript
  (bind _returnvalue (SaveGame|CreateSaveGameObject "/Game/Blueprints/MotionSaveSystem.MotionSaveSystem_C"))
  (Variables|Default|SetSaveMotion _returnvalue)
  (Variables|/Game/Blueprints/MotionSaveSystem.MotionSaveSystem_C|SetsaveGameInstance (Variables|Default|GetSaveMotion) _returnvalue))

(fn FetchCurrentTransforms
  (bind _head (Variables|Default|GetHead))
  (bind _lefthand (Variables|Default|GetLeftHand))
  (bind _righthand (Variables|Default|GetRightHand))
  (bind _returnvalue (Transformation|GetRelativeTransform _righthand))
  (bind _returnvalue_2 (Transformation|GetRelativeTransform _head))
  (bind _returnvalue_3 (Transformation|GetRelativeTransform _lefthand))
  (bind _transformtosave (Utilities|Struct|MakeTransformToSave _returnvalue_2 _returnvalue_3 _returnvalue))
  (bind (_head_2 _left_hand _right_hand) (Utilities|Struct|BreakTransformToSave _transformtosave))
  (Development|PrintString (Utilities|String|Append (Utilities|String|ToString(Transform) _head_2) (Utilities|String|ToString(Transform) _left_hand) (Utilities|String|ToString(Transform) _right_hand)))
  (return _transformtosave))