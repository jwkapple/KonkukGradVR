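; BP_Enemy is an enemy that takes damage, shows its health on a widget bar and dies.
; BeginPlay caches the HP widget as BP_MonsterHP and sets its initial percentage.
; AnyDamage subtracts from HP and updates the bar, then plays a hit montage, or at zero HP a death montage followed by destruction after a short delay.
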(event EventBeginPlay
  (bind _asbp_monster_hp (Utilities|Casting|CastToBP_MonsterHP (UserInterface|GetUserWidgetObject (Variables|Default|GetHPWidget))))
  (bind _output_get (Variables|Default|SetHP_Bar_UI _asbp_monster_hp))
  (Variables|/Game/Blueprints/BP_MonsterHP.BP_MonsterHP_C|SetHPPercent _output_get (/ (Variables|HP|GetHP) (Variables|HP|GetMaxHP))))

(event Collision|EventActorBeginOverlap
  (params (OtherActor :type Actor%20Object%20Reference)))

(event EventTick
  (params (DeltaSeconds :type Float%20%28single-precision%29)))

(event Game|Damage|EventAnyDamage
  (params (Damage :type Float%20%28single-precision%29) (DamageType :type Damage%20Type%20Object%20Reference) (InstigatedBy :type Controller%20Object%20Reference) (DamageCauser :type Actor%20Object%20Reference))
  (Variables|HP|SetHP (- (Variables|HP|GetHP) Damage))
  (Variables|/Game/Blueprints/BP_MonsterHP.BP_MonsterHP_C|SetHPPercent (Variables|Default|GetHP_Bar_UI) (/ (Variables|HP|GetHP) (Variables|HP|GetMaxHP)))
  (if (<= (Variables|HP|GetHP) 0.0)
    (Animation|PlayAnimMontage "/Game/Blueprints/DeadMontage.DeadMontage" 1.0 "None")
    (Utilities|FlowControl|Delay 1.0)
    (Actor|DestroyActor)
    (else
      (Animation|PlayAnimMontage "/Game/Blueprints/OnHitMontage.OnHitMontage" 1.0 "None"))))

(fn ConstructionScript)