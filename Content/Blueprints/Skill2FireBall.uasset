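; Motion-controller fireball skill that charges while Skill 2 is held and fires on release.
; Tick drives start, execute and end from SkillChecker, first spawning a fake projectile at the left hand.
; Circling the right hand around the left grows its effect, detected by a YZ cross-product sign held for three consecutive checks.
; Release deactivates that effect and spawns BP_Fireball ahead in world X, inheriting the charged scale.
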(event EventBeginPlay)

(event EventTick
  (params (DeltaSeconds :type Float%20%28single-precision%29))
  (bind _skillchecker (Variables|Default|GetskillChecker))
  (Utilities|IsValid _skillchecker
    (:Is%20Valid
      (if (Variables|/Game/Blueprints/SkillChecker.SkillChecker_C|GetisSkill2Pressed _skillchecker)
        (if (Variables|Default|GetisInAction)
          (CallFunction|ExecuteSkill)
          (else
            (CallFunction|StartSkill)
            (Variables|Default|SetisInAction true)))
        (elif (Variables|Default|GetisInAction)
          (CallFunction|EndSkill)
          (Variables|Default|SetisInAction false))))))

(fn StartSkill
  (bind _returnvalue (CallFunction|MakeSkillTransform (Variables|Default|GetleftHand)))
  (bind _returnvalue_2 (Game|SpawnActorfromClass "/Game/Blueprints/BP_FakeProjectile.BP_FakeProjectile_C" _returnvalue "Undefined" 0 0))
  (bind _output_get (Variables|Default|Setskill _returnvalue_2))
  (Transformation|SetWorldScale3D (Variables|/Game/Blueprints/BP_FakeProjectile.BP_FakeProjectile_C|GetFX1 _output_get) (Math|Vector|MakeVector 0.15 0.15 0.15))
  (CallFunction|CacheCurrentHands)
  (Variables|Default|Setprev1 false)
  (Variables|Default|Setprev2 false)
  (Variables|Default|Setprev3 false))

(fn EndSkill
  (bind _lefthand (Variables|Default|GetleftHand))
  (bind _returnvalue (Transformation|GetWorldTransform _lefthand))
  (bind (_location _rotation) (Math|Transform|BreakTransform _returnvalue))
  (Components|Activation|SetActive (Variables|/Game/Blueprints/BP_FakeProjectile.BP_FakeProjectile_C|GetFX1 (Variables|Default|Getskill)) false false)
  (Game|SpawnActorfromClass "/Game/Blueprints/BP_Fireball.BP_Fireball_C" (Math|Transform|MakeTransform (+ (+ _location (* (Math|Vector|GetRightVector _rotation) -1e+01)) "50.000000,0,0") "0, 0, 0" (Transformation|GetWorldScale (Variables|/Game/Blueprints/BP_FakeProjectile.BP_FakeProjectile_C|GetFX1 (Variables|Default|Getskill)))) "Undefined" 0 0))

(fn ExecuteSkill
  (bind _result (CallFunction|IsSpinning))
  (if _result
    (CallFunction|IncreaseSize)
    (CallFunction|CacheCurrentHands)))

(fn MakeSkillTransform
  (params (Left%20Hand :type Scene%20Component%20Object%20Reference%20%28by%20ref%29))
  (bind _returnvalue (Transformation|GetWorldTransform Left%20Hand))
  (bind (_location _rotation) (Math|Transform|BreakTransform _returnvalue))
  (return (Math|Transform|MakeTransform (+ _location (* (Math|Vector|GetRightVector _rotation) -1e+01)) "0, 0, 0" "0.100000,0.100000,0.100000")))

(fn IncreaseSize
  (bind _skill (Variables|Default|Getskill))
  (bind _fx1 (Variables|/Game/Blueprints/BP_FakeProjectile.BP_FakeProjectile_C|GetFX1 _skill))
  (Transformation|SetWorldScale3D _fx1 (+ (Transformation|GetWorldScale _fx1) "0.100000,0.100000,0.100000")))

(fn IsSpinning
  (bind _righthand (Variables|Default|GetrightHand))
  (bind _prevrighthand (Variables|Default|GetprevRightHand))
  (bind _lefthand (Variables|Default|GetleftHand))
  (bind _returnvalue (Transformation|GetRelativeTransform _righthand))
  (bind _returnvalue_2 (Transformation|GetRelativeTransform _lefthand))
  (bind _location (Math|Transform|BreakTransform _returnvalue))
  (bind _location_2 (Math|Transform|BreakTransform _returnvalue_2))
  (bind _returnvalue_3 (Math|Vector|GetUnitDirection(Vector) _location_2 _prevrighthand))
  (bind _returnvalue_4 (Math|Vector|GetUnitDirection(Vector) _location_2 _location))
  (bind (_x _y _z) (Math|Vector|BreakVector _returnvalue_4))
  (bind (_x_2 _y_2 _z_2) (Math|Vector|BreakVector _returnvalue_3))
  (bind _returnvalue_5 (Math|Vector2D|MakeVector2D _y _z))
  (bind _returnvalue_6 (Math|Vector2D|MakeVector2D _y_2 _z_2))
  (bind _returnvalue_7 (Class|KismetMathLibrary|CrossProduct2D _returnvalue_6 _returnvalue_5))
  (bind _returnvalue_8 (< _returnvalue_7 0.0))
  (LocalVariables|SetFunctionResult (and (Variables|Default|Getprev2) (and (Variables|Default|Getprev1) _returnvalue_8)))
  (Variables|Default|Setprev3 (Variables|Default|Getprev2))
  (Variables|Default|Setprev2 (Variables|Default|Getprev1))
  (Variables|Default|Setprev1 _returnvalue_8)
  (Development|PrintString (Utilities|String|ToString(Boolean) _returnvalue_8))
  (return (LocalVariables|GetFunctionResult)))

(fn CacheCurrentHands
  (Variables|Default|SetprevLeftHand (.Location (Math|Transform|BreakTransform (Transformation|GetRelativeTransform (Variables|Default|GetleftHand)))))
  (Variables|Default|SetprevRightHand (.Location (Math|Transform|BreakTransform (Transformation|GetRelativeTransform (Variables|Default|GetrightHand))))))

(fn IsHigherThenPrev
  (params (controller :type Scene%20Component%20Object%20Reference) (prevController :type Vector))
  (Math|Float|CompareFloat (+ (.X (Math|Vector|BreakVector prevController)) (Variables|Default|GetmagicHeight)) (.X (Math|Vector|BreakVector (.Location (Math|Transform|BreakTransform (Transformation|GetRelativeTransform controller)))))
    (:>
      _)
    (:==
      _)
    (:<
      (return true)))
  (return false))