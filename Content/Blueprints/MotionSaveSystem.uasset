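; MotionSaveSystem saves and loads motion Sequences in named save-game slots.
; SaveMotion writes the Sequences into SaveGameInstance and saves it to the given slot.
; LoadMotion checks the slot exists, casts the loaded object to MotionSaveSystem, caches it as SaveGameInstance and returns its Sequences.
; Both print Korean status messages, with red warnings for failed saves, missing files, or corrupted or outdated saves; SaveGameInstance is not created in these functions.
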(fn SaveMotion
  (params (sequences :type Array%20of%20Sequence%20to%20Save%20Structures) (saveFileName :type String))
  (bind _savegameinstance (Variables|Default|GetsaveGameInstance))
  (Variables|MotionSaveSystem_C|Setsequences _savegameinstance sequences)
  (bind _returnvalue (SaveGame|SaveGametoSlot _savegameinstance saveFileName))
  (if _returnvalue
    (Development|PrintString 0 (Utilities|String|Append "[Log] 저장 성공. 파일명: " saveFileName) true true "(R=0.000000,G=0.660000,B=1.000000,A=1.000000)" 5.0)
    (else
      (Development|PrintString 0 (Utilities|String|Append "[Warning] 저장 실패. 입력한 파일명: " saveFileName) true true "(R=1.000000,G=0.000000,B=0.000000,A=1.000000)" 5.0))))

(fn LoadMotion
  (params (saveFileName :type String))
  (bind _returnvalue (SaveGame|DoesSaveGameExist saveFileName))
  (if _returnvalue
    (bind _returnvalue_2 (SaveGame|LoadGamefromSlot saveFileName))
    (bind _asmotion_save_system (Utilities|Casting|CastToMotionSaveSystem _returnvalue_2)
      (:then
        (bind _output_get (Variables|Default|SetsaveGameInstance _asmotion_save_system))
        (Development|PrintString 0 (Utilities|String|Append "[Log] 로드 성공. 불러온 파일명: " saveFileName) true true "(R=0.000000,G=0.660000,B=1.000000,A=1.000000)" 5.0)
        (return (Variables|MotionSaveSystem_C|Getsequences _output_get)))
      (:CastFailed
        (Development|PrintString 0 (Utilities|String|Append "[Warning] 로드 실패. 파일이 손상되었거나 예전 버전임: " saveFileName) true true "(R=1.000000,G=0.000000,B=0.000000,A=1.000000)" 5.0)))
    (else
      (Development|PrintString 0 (Utilities|String|Append "[Warning] 로드 실패. 파일 이름을 정확히 입력했는 지 확인 바람. 입력한 파일명: " saveFileName) true true "(R=1.000000,G=0.000000,B=0.000000,A=1.000000)" 5.0))))