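; Thunder skill driven by head and hand motion, casting a storm cloud on a targeted pawn while SkillChecker reports Skill 1 pressed.
; On press, a downward-angled line trace from the head picks the pawn and spawns BP_Cloud above it.
; While held, Tick grows the cloud effect when both hands drop relative to last frame, offset by MagicHeight.
; Release deactivates the cloud, then triggers lightning, fixed damage and an explosion sound.
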(event EventBeginPlay)

(event EventTick
  (params (DeltaSeconds :type Float%20%28single-precision%29))
  (bind _skillchecker (Variables|Default|GetskillChecker))
  (Utilities|IsValid _skillchecker
    (:Is%20Valid
      (if (Variables|/Game/Blueprints/SkillChecker.SkillChecker_C|GetisSkill1Pressed _skillchecker)
        (if (Variables|Default|GetisInAction)
          (CallFunction|ExecuteSkill)
          (else
            (CallFunction|StartSkill)
            (Variables|Default|SetisInAction true)))
        (elif (Variables|Default|GetisInAction)
          (CallFunction|EndSkill)
          (Variables|Default|SetisInAction false))))))

(fn StartSkill
  (bind _head (Variables|Default|Gethead))
  (bind _returnvalue (Transformation|GetWorldTransform _head))
  (Development|PrintString "start")
  (bind _outhit (Collision|LineTraceForObjects (.location _returnvalue) (- (+ (.location _returnvalue) (* (Math|Vector|GetForwardVector (.rotation _returnvalue)) "3000.000000,3000.000000,3000.000000")) "0,0,500.000000") (Utilities|Array|MakeArray "ObjectTypeQuery3") false 0 "ForDuration"))
  (Variables|Default|SetHit%20Actor (.HitActor (Collision|BreakHitResult _outhit)))
  (bind _output_get (Variables|Default|SetMonsterLocation (Math|Transform|MakeTransform (+ (Transformation|GetActorLocation (.HitActor (Collision|BreakHitResult _outhit))) "0,0,350.000000"))))
  (bind _returnvalue_2 (Game|SpawnActorfromClass "/Game/Blueprints/BP_Cloud.BP_Cloud_C" _output_get "Undefined" 0 0))
  (bind _output_get_2 (Variables|Default|Setskill _returnvalue_2))
  (Transformation|SetWorldScale3D (Variables|/Game/Blueprints/BP_FakeProjectile.BP_FakeProjectile_C|GetFX1 _output_get_2) (Math|Vector|MakeVector 0.7 0.7 0.7))
  (CallFunction|CacheCurrentHands))

(fn EndSkill
  (bind _hit_actor (Variables|Default|GetHit%20Actor))
  (Components|Activation|SetActive (Variables|/Game/Blueprints/BP_FakeProjectile.BP_FakeProjectile_C|GetFX1 (Variables|Default|Getskill)) false false)
  (Effects|SpawnEmitteratLocation "/Game/FXVarietyPack/Particles/P_ky_lightning3.P_ky_lightning3" (- (.location (Variables|Default|GetMonsterLocation)) "0,0,600.000000"))
  (Game|Damage|ApplyDamage _hit_actor 1e+01 0 0)
  (Audio|SpawnSoundatLocation "/Game/StarterContent/Audio/Explosion01.Explosion01" (Transformation|GetActorLocation _hit_actor) "0, 0, 0" 1.0 1.0 0.0 0 0))

(fn ExecuteSkill
  (bind _result (CallFunction|IsControllerDecreasing))
  (if _result
    (CallFunction|IncreaseSize))
  (CallFunction|CacheCurrentHands))

(fn MakeSkillTransform
  (params (head :type Scene%20Component%20Object%20Reference%20%28by%20ref%29))
  (bind _returnvalue (Transformation|GetWorldTransform head))
  (bind (_location _rotation) (Math|Transform|BreakTransform _returnvalue))
  (bind _returnvalue_2 (Math|Vector|GetForwardVector _rotation))
  (bind _returnvalue_3 (* _returnvalue_2 5e+02))
  (bind _returnvalue_4 (+ _location _returnvalue_3))
  (bind (_x _y) (Math|Vector|BreakVector _returnvalue_4))
  (bind _returnvalue_5 (Math|Vector|MakeVector _x _y 0.0))
  (bind _returnvalue_6 (Math|Transform|MakeTransform _returnvalue_5))
  (Development|PrintString (Utilities|String|ToString(Transform) _returnvalue_6))
  (return _returnvalue_6))

(fn IncreaseSize
  (bind _skill (Variables|Default|Getskill))
  (bind _fx1 (Variables|/Game/Blueprints/BP_FakeProjectile.BP_FakeProjectile_C|GetFX1 _skill))
  (Transformation|SetWorldScale3D _fx1 (+ (Transformation|GetWorldScale _fx1) "0.100000,0.100000,0.100000")))

(fn IsControllerDecreasing
  (bind _result (CallFunction|IsLowerThenPrev (Variables|Default|GetleftHand) (Variables|Default|GetprevLeftHand)))
  (bind _result_2 (CallFunction|IsLowerThenPrev (Variables|Default|GetrightHand) (Variables|Default|GetprevRightHand)))
  (return (and _result _result_2)))

(fn CacheCurrentHands
  (Variables|Default|SetprevLeftHand (.Location (Math|Transform|BreakTransform (Transformation|GetRelativeTransform (Variables|Default|GetleftHand)))))
  (Variables|Default|SetprevRightHand (.Location (Math|Transform|BreakTransform (Transformation|GetRelativeTransform (Variables|Default|GetrightHand))))))

(fn IsLowerThenPrev
  (params (controller :type Scene%20Component%20Object%20Reference) (prevController :type Vector))
  (Math|Float|CompareFloat (+ (.Z (Math|Vector|BreakVector prevController)) (Variables|Default|GetmagicHeight)) (.Z (Math|Vector|BreakVector (.Location (Math|Transform|BreakTransform (Transformation|GetRelativeTransform controller)))))
    (:>
      (return true))
    (:==
      _)
    (:<
      _))
  (return false))