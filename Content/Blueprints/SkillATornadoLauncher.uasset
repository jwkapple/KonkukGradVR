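; Tornado skill launcher that spawns and grows a BP_Tornado while SkillChecker reports Skill 4 pressed.
; Tick tracks press and release through IsInAction, spawning the tornado offset along X from the player head's relative location at Z zero.
; Its effect starts nearly flat and stretches vertically by a fixed step each held frame, independent of delta time.
; EndSkill is empty, so release just stops the growth.
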(event EventBeginPlay)

(event EventTick
  (params (DeltaSeconds :type Float%20%28single-precision%29))
  (if (Variables|/Game/Blueprints/SkillChecker.SkillChecker_C|GetisSkill4Pressed (Variables|Default|GetskillChecker))
    (if (Variables|Default|GetisInAction)
      (CallFunction|ExecuteSkill)
      (else
        (CallFunction|StartSkill)
        (Variables|Default|SetisInAction true)))
    (elif (Variables|Default|GetisInAction)
      (CallFunction|EndSkill)
      (Variables|Default|SetisInAction false))))

(fn StartSkill
  (bind _returnvalue (CallFunction|MakeSkillTransform (Transformation|GetRelativeTransform (Variables|/Game/Blueprints/MotionPlayer.MotionPlayer_C|GetHead (Variables|Default|Getplayer)))))
  (bind _returnvalue_2 (Game|SpawnActorfromClass "/Game/Blueprints/BP_Tornado.BP_Tornado_C" _returnvalue "Undefined" 0 0))
  (bind _output_get (Variables|Default|Setskill _returnvalue_2))
  (Transformation|SetWorldScale3D (Variables|/Game/FXVarietyPack/Blueprints/BP_ky_storm.BP_ky_storm_C|Getfx _output_get) (Math|Vector|MakeVector 1.0 1.0 0.01)))

(fn EndSkill)

(fn ExecuteSkill
  (bind _skill (Variables|Default|Getskill))
  (bind _fx (Variables|/Game/FXVarietyPack/Blueprints/BP_ky_storm.BP_ky_storm_C|Getfx _skill))
  (bind _returnvalue (Transformation|GetWorldScale _fx))
  (bind (_x _y _z) (Math|Vector|BreakVector _returnvalue))
  (Transformation|SetWorldScale3D _fx (Math|Vector|MakeVector _x _y (+ _z 0.05))))

(fn MakeSkillTransform
  (params (InTransform :type Transform%20%28by%20ref%29))
  (bind _location (Math|Transform|BreakTransform InTransform))
  (bind (_x _y) (Math|Vector|BreakVector _location))
  (return (Math|Transform|MakeTransform (Math|Vector|MakeVector (+ _x 1e+02) _y 0.0))))