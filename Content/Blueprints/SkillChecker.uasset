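; SkillChecker picks one of four skill flags from VR trigger input and hand-to-head distance.
; Check requires exactly one pressed trigger, then compares that hand's distance to CenterRadius to choose between its two skills, otherwise clearing all flags.
; The GetDistanceHeadToCon call supplying those distances is off the execution path, so it never runs.
; Tick prints the active skill as on-screen debug text.
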(event EventBeginPlay)

(event EventTick
  (params (DeltaSeconds :type Float%20%28single-precision%29))
  (if (Variables|Default|GetisSkill1Pressed)
    (Variables|Default|Setprint (Utilities|String|MakeLiteralString "Skill 1 is pressed"))
    (Development|PrintString (Variables|Default|Getprint) true false "(R=0.000000,G=0.660000,B=1.000000,A=1.000000)" 0.05 :!label _label)
    (elif (Variables|Default|GetisSkill2Pressed)
      (Variables|Default|Setprint (Utilities|String|MakeLiteralString "Skill 2 is pressed"))
      (goto _label)
      (elif (Variables|Default|GetisSkill3Pressed)
        (Variables|Default|Setprint (Utilities|String|MakeLiteralString "Skill 3 is pressed"))
        (goto _label)
        (elif (Variables|Default|GetisSkill4Pressed)
          (Variables|Default|Setprint (Utilities|String|MakeLiteralString "Skill 4 is pressed"))
          (goto _label))))))

(fn Check
  (params (head :type Transform) (leftHand :type Transform) (rightHand :type Transform) (isLeftTriggerPressed :type Boolean) (isRightTriggerPressed :type Boolean))
  (if (Class|KismetMathLibrary|XORBoolean isLeftTriggerPressed isRightTriggerPressed)
    (if isLeftTriggerPressed
      (Math|Float|CompareFloat (stale _headtolefthand) (LocalVariables|GetcenterRadius)
        (:>
          (Variables|Default|SetisSkill1Pressed true)
          (Variables|Default|SetisSkill2Pressed false))
        (:==
          (Variables|Default|SetisSkill1Pressed false :!label _label)
          (Variables|Default|SetisSkill2Pressed true))
        (:<
          (goto _label)))
      (elif isRightTriggerPressed
        (Math|Float|CompareFloat (stale _headtorighthand) (LocalVariables|GetcenterRadius)
          (:>
            (Variables|Default|SetisSkill3Pressed false)
            (Variables|Default|SetisSkill4Pressed true))
          (:==
            (Variables|Default|SetisSkill3Pressed true :!label _label_2)
            (Variables|Default|SetisSkill4Pressed false))
          (:<
            (goto _label_2)))))
    (else
      (Variables|Default|SetisSkill1Pressed false)
      (Variables|Default|SetisSkill2Pressed false)
      (Variables|Default|SetisSkill3Pressed false)
      (Variables|Default|SetisSkill4Pressed false))))

(fn GetDistanceHeadtoCon
  (params (head :type Transform) (leftHand :type Transform) (rightHand :type Transform))
  (bind _location (Math|Transform|BreakTransform head))
  (return (Math|Vector|Distance(Vector) _location (.Location (Math|Transform|BreakTransform leftHand))) (Math|Vector|Distance(Vector) _location (.Location (Math|Transform|BreakTransform rightHand)))))