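; Motion playback actor that replays recorded head, hand and trigger sequences, loaded and re-saved through a MotionSaveSystem object.
; Index or random playback validates the data, then Tick applies one snapshot per frame until the sequence ends.
; Each step passes the next snapshot to SkillChecker and tints the hands red while their triggers are pressed.
; The construction script wires the checker and body parts into the tornado, three-ball and fireball skills.
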(event Custom|LoadRecords
  (bind _sequences (Default|LoadMotion (Variables|Default|GetSaveMotion) (Variables|Default|GetsaveFileName)))
  (Variables|Default|Setsequences _sequences))

(event Custom|PlayByIndex
  (CallFunction|ForceStop)
  (bind _validation (CallFunction|ValidateData))
  (if _validation
    (bind _validation_2 (CallFunction|ValidateIndex))
    (if _validation_2
      (Variables|Default|SetIsPlaying true))))

(event Custom|re-save
  (Default|SaveMotion (Variables|Default|GetSaveMotion) (Variables|Default|Getsequences) (Variables|Default|GetsaveFileName)))

(event Custom|ForceStop
  (Variables|Default|SetIsPlaying false)
  (Variables|Default|SetcurrentTransformIndex 0))

(event Custom|RandomPlay
  (bind _validation (CallFunction|ValidateData))
  (if _validation
    (Variables|Default|SetsequenceIndex (Math|Random|RandomInteger (+ (Utilities|Array|LastIndex (Variables|Default|Getsequences)) 1)))
    (CallFunction|PlaybyIndex)))

(event EventBeginPlay)

(event Collision|EventActorBeginOverlap
  (params (OtherActor :type Actor%20Object%20Reference)))

(event EventTick
  (params (DeltaSeconds :type Float%20%28single-precision%29))
  (if (Variables|Default|GetIsPlaying)
    (CallFunction|PlayMotion (Variables|Default|GetsequenceIndex))))

(fn ConstructionScript
  (bind _self self)
  (bind _skill3ball (Variables|Default|GetSkill3Ball))
  (bind _skill1fireball (Variables|Default|GetSkill1FireBall))
  (bind _skillatornadolauncher (Variables|Default|GetSkillATornadoLauncher))
  (bind _returnvalue (SaveGame|CreateSaveGameObject "/Game/Blueprints/MotionSaveSystem.MotionSaveSystem_C"))
  (Variables|Default|SetSaveMotion _returnvalue)
  (Variables|/Game/Blueprints/MotionSaveSystem.MotionSaveSystem_C|SetsaveGameInstance (Variables|Default|GetSaveMotion) _returnvalue)
  (bind _output_get (Variables|/Game/Blueprints/SkillATornadoLauncher.SkillATornadoLauncher_C|SetskillChecker _skillatornadolauncher (Variables|Default|GetSkillChecker)))
  (bind _output_get_2 (Variables|/Game/Blueprints/SkillATornadoLauncher.SkillATornadoLauncher_C|Sethead _skillatornadolauncher (Variables|Default|GetHead _self)))
  (bind _output_get_3 (Variables|/Game/Blueprints/SkillATornadoLauncher.SkillATornadoLauncher_C|SetleftHand _skillatornadolauncher (Variables|Default|GetLeftHand _self)))
  (bind _output_get_4 (Variables|/Game/Blueprints/SkillATornadoLauncher.SkillATornadoLauncher_C|SetrightHand _skillatornadolauncher (Variables|Default|GetRightHand _self)))
  (bind _output_get_5 (Variables|/Game/Blueprints/Skill3Ball.Skill3Ball_C|SetskillChecker _skill3ball _output_get))
  (bind _output_get_6 (Variables|/Game/Blueprints/Skill3Ball.Skill3Ball_C|Sethead _skill3ball _output_get_2))
  (bind _output_get_7 (Variables|/Game/Blueprints/Skill3Ball.Skill3Ball_C|SetleftHand _skill3ball _output_get_3))
  (bind _output_get_8 (Variables|/Game/Blueprints/Skill3Ball.Skill3Ball_C|SetrightHand _skill3ball _output_get_4))
  (Variables|/Game/Blueprints/Skill1FireBall.Skill1FireBall_C|SetskillChecker _skill1fireball _output_get_5)
  (Variables|/Game/Blueprints/Skill1FireBall.Skill1FireBall_C|Sethead _skill1fireball _output_get_6)
  (Variables|/Game/Blueprints/Skill1FireBall.Skill1FireBall_C|SetleftHand _skill1fireball _output_get_7)
  (Variables|/Game/Blueprints/Skill1FireBall.Skill1FireBall_C|SetrightHand _skill1fireball _output_get_8))

(fn PlayMotion
  (params (sequenceIndex :type Integer))
  (bind _righthand (Variables|Default|GetRightHand))
  (bind _lefthand (Variables|Default|GetLeftHand))
  (bind _sequences (Variables|Default|Getsequences))
  (bind _output (Utilities|Array|Get(acopy) _sequences sequenceIndex))
  (bind _snapshots (Utilities|Struct|BreakSequenceToSave _output))
  (Math|Integer|CompareInt (Variables|Default|GetcurrentTransformIndex) (Utilities|Array|LastIndex _snapshots)
    (:>
      (CallFunction|ForceStop :!label _label)
      (Development|PrintString "[Log] 재생 종료" true true "(R=0.000000,G=0.660000,B=1.000000,A=1.000000)" 5.0))
    (:==
      (goto _label))
    (:<
      (CallFunction|SetCurrentSnapshot (.head (Utilities|Struct|BreakSnapshot (Utilities|Array|Get(acopy) _snapshots (Variables|Default|GetcurrentTransformIndex)))) (.left_hand (Utilities|Struct|BreakSnapshot (Utilities|Array|Get(acopy) _snapshots (Variables|Default|GetcurrentTransformIndex)))) (.right_hand (Utilities|Struct|BreakSnapshot (Utilities|Array|Get(acopy) _snapshots (Variables|Default|GetcurrentTransformIndex)))) (.is_left_trigger_pressed (Utilities|Struct|BreakSnapshot (Utilities|Array|Get(acopy) _snapshots (Variables|Default|GetcurrentTransformIndex)))) (.is_right_trigger_pressed (Utilities|Struct|BreakSnapshot (Utilities|Array|Get(acopy) _snapshots (Variables|Default|GetcurrentTransformIndex)))))
      (Variables|Default|SetcurrentTransformIndex (+ (Variables|Default|GetcurrentTransformIndex) 1))
      (Default|Check (Variables|Default|GetSkillChecker) (Utilities|Array|Get(acopy) _snapshots (Variables|Default|GetcurrentTransformIndex)))
      (if (.is_left_trigger_pressed (Utilities|Struct|BreakSnapshot (Utilities|Array|Get(acopy) _snapshots (Variables|Default|GetcurrentTransformIndex))))
        (Rendering|Material|SetMaterial _lefthand 0 (LocalVariables|Getred))
        (else
          (Rendering|Material|SetMaterial _lefthand 0 (LocalVariables|Getwhite))))
      (if (.is_right_trigger_pressed (Utilities|Struct|BreakSnapshot (Utilities|Array|Get(acopy) _snapshots (Variables|Default|GetcurrentTransformIndex))))
        (Rendering|Material|SetMaterial _righthand 0 (LocalVariables|Getred))
        (else
          (Rendering|Material|SetMaterial _righthand 0 (LocalVariables|Getwhite)))))))

(fn SetCurrentSnapshot
  (params (head :type Transform) (leftHand :type Transform) (rightHand :type Transform) (isLeftTriggerPressed :type Boolean) (isRightTriggerPressed :type Boolean))
  (bind (_location _rotation) (Math|Transform|BreakTransform head))
  (bind (_location_2 _rotation_2) (Math|Transform|BreakTransform leftHand))
  (bind (_location_3 _rotation_3) (Math|Transform|BreakTransform rightHand))
  (Transformation|SetRelativeLocationAndRotation (Variables|Default|GetHead) _location _rotation false false)
  (Transformation|SetRelativeLocationAndRotation (Variables|Default|GetLeftHand) _location_2 _rotation_2 false false)
  (Transformation|SetRelativeLocationAndRotation (Variables|Default|GetRightHand) _location_3 _rotation_3 false false)
  (Variables|Default|SetisLeftTriggerPressed isLeftTriggerPressed)
  (Variables|Default|SetisRightTriggerPressed isRightTriggerPressed)
  (return))

(fn ValidateData
  (if (Utilities|Array|IsEmpty (Variables|Default|Getsequences))
    (Development|PrintString "[Warning] 파일이 로드되지 않았거나, 녹화된 데이터가 없습니다." true true "(R=1.000000,G=0.000000,B=0.000000,A=1.000000)" 5.0)
    (return false)
    (else
      (return true))))

(fn ValidateIndex
  (bind _sequenceindex (Variables|Default|GetsequenceIndex))
  (Math|Integer|CompareInt _sequenceindex (Utilities|Array|LastIndex (Variables|Default|Getsequences))
    (:>
      _)
    (:==
      (Math|Integer|CompareInt _sequenceindex :!label _label
        (:>
          (return true))
        (:==
          (return true))
        (:<
          _)))
    (:<
      (goto _label)))
  (Development|PrintString "[Warning] Sequence Index가 잘못되었습니다." true true "(R=1.000000,G=0.000000,B=0.000000,A=1.000000)" 5.0)
  (return false))