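; Skill 3 logic for a motion-controller water ball that grows as the hands make a circling gesture.
; Tick follows SkillChecker's pressed flag, spawning a small BP_WaterBall beside the right hand, updating it while held and deactivating its effect on release.
; Spin detection uses a 2D cross product of left-hand movement around the right hand in the YZ plane.
; Four consecutive same-direction frames are required before the effect scales up.
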(event EventBeginPlay)

(event EventTick
  (params (DeltaSeconds :type Float%20%28single-precision%29))
  (if (Variables|/Game/Blueprints/SkillChecker.SkillChecker_C|GetisSkill3Pressed (Variables|Default|GetskillChecker))
    (if (Variables|Default|GetisInAction)
      (CallFunction|ExecuteSkill)
      (else
        (CallFunction|StartSkill)
        (Variables|Default|SetisInAction true)))
    (elif (Variables|Default|GetisInAction)
      (CallFunction|EndSkill)
      (Variables|Default|SetisInAction false))))

(fn StartSkill
  (bind _returnvalue (|SpawnBall))
  (Utilities|Array|Resize _returnvalue (Math|Vector|MakeVector 0.1 0.1 0.1))
  (CallFunction|CacheCurrentHands)
  (Variables|Default|Setprev1 false)
  (Variables|Default|Setprev2 false)
  (Variables|Default|Setprev3 false))

(fn EndSkill
  (Components|Activation|SetActive (Variables|/Game/FXVarietyPack/Blueprints/BP_ky_storm.BP_ky_storm_C|Getfx (Variables|Default|Getskill)) false false))

(fn ExecuteSkill
  (bind _result (CallFunction|IsSpinning))
  (if _result
    (CallFunction|IncreaseSize))
  (CallFunction|CacheCurrentHands))

(fn MakeSkillTransform
  (params (rightHand :type Scene%20Component%20Object%20Reference%20%28by%20ref%29))
  (bind _returnvalue (Transformation|GetWorldTransform rightHand))
  (bind (_location _rotation) (Math|Transform|BreakTransform _returnvalue))
  (return (Math|Transform|MakeTransform (+ _location (* (Math|Vector|GetRightVector _rotation) -1e+01)))))

(fn IncreaseSize
  (bind _skill (Variables|Default|Getskill))
  (bind _fx (Variables|/Game/FXVarietyPack/Blueprints/BP_ky_storm.BP_ky_storm_C|Getfx _skill))
  (Transformation|SetWorldScale3D _fx (+ (Transformation|GetWorldScale _fx) "0.030000,0.030000,0.030000")))

(fn IsSpinning
  (bind _righthand (Variables|Default|GetrightHand))
  (bind _prevlefthand (Variables|Default|GetprevLeftHand))
  (bind _lefthand (Variables|Default|GetleftHand))
  (bind _returnvalue (Transformation|GetRelativeTransform _lefthand))
  (bind _returnvalue_2 (Transformation|GetRelativeTransform _righthand))
  (bind _location (Math|Transform|BreakTransform _returnvalue))
  (bind _location_2 (Math|Transform|BreakTransform _returnvalue_2))
  (bind _returnvalue_3 (Math|Vector|GetUnitDirection(Vector) _location_2 _prevlefthand))
  (bind _returnvalue_4 (Math|Vector|GetUnitDirection(Vector) _location_2 _location))
  (bind (_x _y _z) (Math|Vector|BreakVector _returnvalue_4))
  (bind (_x_2 _y_2 _z_2) (Math|Vector|BreakVector _returnvalue_3))
  (bind _returnvalue_5 (Math|Vector2D|MakeVector2D _y _z))
  (bind _returnvalue_6 (Math|Vector2D|MakeVector2D _y_2 _z_2))
  (bind _returnvalue_7 (- _returnvalue_5 _returnvalue_6))
  (bind _returnvalue_8 (- "" _returnvalue_6))
  (bind _returnvalue_9 (Class|KismetMathLibrary|CrossProduct2D _returnvalue_8 _returnvalue_7))
  (bind _returnvalue_10 (< _returnvalue_9 0.0))
  (LocalVariables|SetfunctionResult (and (and (Variables|Default|Getprev3) (Variables|Default|Getprev2)) (and (Variables|Default|Getprev1) _returnvalue_10)))
  (Variables|Default|Setprev3 (Variables|Default|Getprev2))
  (Variables|Default|Setprev2 (Variables|Default|Getprev1))
  (Variables|Default|Setprev1 _returnvalue_10)
  (return (LocalVariables|GetfunctionResult)))

(fn CacheCurrentHands
  (Variables|Default|SetprevLeftHand (.Location (Math|Transform|BreakTransform (Transformation|GetRelativeTransform (Variables|Default|GetleftHand)))))
  (Variables|Default|SetprevRightHand (.Location (Math|Transform|BreakTransform (Transformation|GetRelativeTransform (Variables|Default|GetrightHand))))))

(fn IsHigherThenPrev
  (params (controller :type Scene%20Component%20Object%20Reference) (prevController :type Vector))
  (Math|Float|CompareFloat (+ (.Z (Math|Vector|BreakVector prevController)) (Variables|Default|GetmagicHeight)) (.Z (Math|Vector|BreakVector (.Location (Math|Transform|BreakTransform (Transformation|GetRelativeTransform controller)))))
    (:>
      _)
    (:==
      _)
    (:<
      (return true)))
  (return false))